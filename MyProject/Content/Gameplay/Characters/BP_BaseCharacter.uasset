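; Base fighter for a side-view, card-driven combat game, moving along Y on a PaperZD-animated sprite.
; Commands are either numeric steps, setting speed and facing-relative state for Tick movement, or skill names, loading attack data and animation from GameDirector.
; Attacks box-trace for the enemy and apply health and Ren changes, softened while moving, pushing reaction states to BaseMaster.
; Helpers handle move-range limits, target markers, turning and pausing.
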(event `self.ReceiveBeginPlay`)

(event `self.ReceiveTick`
  (params (DeltaSeconds :type "Float (single-precision)"))
  (if (not (`self.HasStop`))
    (`self.UpdateMove` DeltaSeconds)))

(fn `Attacked`
  (params (Health :type "Float (double-precision)") (Ren :type "Float (double-precision)"))
  (returns (IsOk :type Boolean))
  (locals (RealDeltaHealth :type "Float (double-precision)") (RealDeltaRen :type "Float (double-precision)"))
  (switch `/Game/Gameplay/Characters/E_CharacterState` (`self.CharacterState`)
    (:`NewEnumerator0`
      (set `local.RealDeltaHealth` Health)
      (set `local.RealDeltaRen` Ren))
    (:`NewEnumerator1`
      (set `local.RealDeltaHealth` (/ Health 2.0) :!label _label)
      (set `local.RealDeltaRen` 0.0)
      (`/Game/Gameplay/BattleFields/Master/BP_BaseMaster.InsertState` (`self.BaseMaster`) "NewEnumerator3"))
    (:`NewEnumerator2`
      (goto _label)))
  (bind _output_get (set `self.CurrentHealth` (`KismetMathLibrary.FMax` (+ (`self.CurrentHealth`) (`local.RealDeltaHealth`)))))
  (if (<= _output_get 0.0)
    (`KismetSystemLibrary.PrintString` "One Characte Dead!")
    (return false)
    (elif (`|EnumInequality` (`self.CharacterState`) "NewEnumerator3")
      (bind _newren (`self.SetRen` (`local.RealDeltaRen`)))
      (`/Game/Gameplay/BattleFields/Master/BP_BaseMaster.InsertState` (`self.BaseMaster`) "NewEnumerator1")
      (if (<= _newren 0.0)
        (`/Game/Gameplay/BattleFields/Master/BP_BaseMaster.InsertState` (`self.BaseMaster`) "NewEnumerator2"))
      (return true))))

(fn `ChangeFaceDirection`
  (bind (_facedirection_x _facedirection_y) (`KismetMathLibrary.BreakVector` (`self.FaceDirection`)))
  (bind (_returnvalue_x _returnvalue_y) (`KismetMathLibrary.BreakVector` (`SceneComponent.K2_GetComponentLocation` (`self.CapsuleComponent`))))
  (bind (_returnvalue_x_2 _returnvalue_y_2) (`KismetMathLibrary.BreakVector` (`SceneComponent.K2_GetComponentLocation` (`Character.CapsuleComponent` (`self.EnemyCharacter`)))))
  (if (<= (* _facedirection_y (- _returnvalue_y_2 _returnvalue_y)) 0.0)
    (set `self.FaceDirection` (* (`self.FaceDirection`) (0.0 -1.0 0.0)))
    (`self.K2_AddActorWorldRotation` (struct :`Yaw` 180.0))))

(fn `ChangeMoveAttention`
  (params (Index :type Integer))
  (bind _moveattention (`self.MoveAttention`))
  (bind (_returnvalue_x _returnvalue_y _returnvalue_z) (`KismetMathLibrary.BreakVector` (`SceneComponent.K2_GetComponentLocation` (`self.CapsuleComponent`))))
  (`/Engine/EditorBlueprintResources/StandardMacros.IsValid` _moveattention
    (:`Is Valid`
      (`self.K2_DestroyActor` _moveattention)
      (set `self.MoveAttention` null))
    (:`Is Not Valid`
      _))
  (if (not (== Index 0))
    (bind _returnvalue (`|SpawnActorFromClass` "/Script/Engine.StaticMeshActor" (`KismetMathLibrary.MakeTransform` (`KismetMathLibrary.MakeVector` (+ _returnvalue_x 100.0) (+ _returnvalue_y (* (`self.MoveStep`) Index)) (- _returnvalue_z 130.0)) (struct :`Pitch` -90.0) (1.0 1.2 1.0)) "AlwaysSpawn" "MultiplyWithRoot" null null))
    (bind _staticmeshcomponent (`StaticMeshActor.StaticMeshComponent` _returnvalue))
    (`SceneComponent.SetMobility` _staticmeshcomponent "Movable")
    (`StaticMeshComponent.SetStaticMesh` _staticmeshcomponent "/Game/Gameplay/Characters/Other/SM_MoveAttention.SM_MoveAttention")
    (set `self.MoveAttention` _returnvalue)))

(fn `ExecuteAttack`
  (bind _attackinfo (`self.AttackInfo`))
  (bind (_facedirection_x _facedirection_y) (`KismetMathLibrary.BreakVector` (`self.FaceDirection`)))
  (bind (_attackinfo_boxposition _attackinfo_boxsize _attackinfo_attackvalue _attackinfo_renvalue) (break `/Game/Gameplay/Cards/Skills/S_AttackInfo` (`self.AttackInfo`)))
  (bind (_returnvalue_x _returnvalue_y _returnvalue_z) (`KismetMathLibrary.BreakVector` (`SceneComponent.K2_GetComponentLocation` (`self.CapsuleComponent`))))
  (bind _returnvalue (+ _returnvalue_z (`.Y` (`KismetMathLibrary.BreakVector2D` (break `/Game/Gameplay/Cards/Skills/S_AttackInfo` _attackinfo)))))
  (bind _returnvalue_2 (+ _returnvalue_y (* (`KismetMathLibrary.BreakVector2D` (break `/Game/Gameplay/Cards/Skills/S_AttackInfo` _attackinfo)) _facedirection_y)))
  (bind _outhits (`KismetSystemLibrary.BoxTraceMultiForObjects` :`Start` (`KismetMathLibrary.MakeVector` _returnvalue_x _returnvalue_2 _returnvalue) :`End` (`KismetMathLibrary.MakeVector` _returnvalue_x _returnvalue_2 _returnvalue) :`HalfSize` (`KismetMathLibrary.MakeVector` 32.0 (/ (`KismetMathLibrary.BreakVector2D` (`.BoxSize_8_F78634924A01CC86215E168912E6FF08` (break `/Game/Gameplay/Cards/Skills/S_AttackInfo` _attackinfo))) 2.0) (/ (`.Y` (`KismetMathLibrary.BreakVector2D` (`.BoxSize_8_F78634924A01CC86215E168912E6FF08` (break `/Game/Gameplay/Cards/Skills/S_AttackInfo` _attackinfo)))) 2.0)) :`ObjectTypes` (`|MakeArray` "ObjectTypeQuery8" :!type "EObjectTypeQuery Enum") :`DrawTime` 1.0))
  (for _array_element _outhits
    (bind _asbp_base_character (cast `/Game/Gameplay/Characters/BP_BaseCharacter` (`.HitActor` (`GameplayStatics.BreakHitResult` _array_element))))
    (if (== _asbp_base_character (`self.EnemyCharacter`))
      (`self.Attacked` (`self.EnemyCharacter`) _attackinfo_attackvalue _attackinfo_renvalue))))

(fn `ExecuteCommand`
  (params (Command :type String))
  (bind _returnvalue (`KismetStringLibrary.Conv_StringToInt` Command))
  (bind (_facedirection_x _facedirection_y) (`KismetMathLibrary.BreakVector` (`self.FaceDirection`)))
  (bind (_skillinfo_animseq _skillinfo_ke _skillinfo_attackinfoarray) (break `/Game/Gameplay/Cards/Skills/S_SkillInfo` (`/Game/Gameplay/Cards/BP_CardInfo.Get Skill Info` (`/Game/Gameplay/Director/GameDirector.TotalCardInfo` (`self.GameDirector`)) Command (`self.CharacterType`))))
  (if (`KismetStringLibrary.IsNumeric` Command)
    (if (!= _returnvalue 0)
      (bind _output_get (set `self.MoveSpeed` (`KismetMathLibrary.Conv_IntToDouble` (* (/ (`self.MoveStep`) (`/Game/Gameplay/BattleFields/Master/BP_BaseMaster.KeInterval` (`self.BaseMaster`))) (/ _returnvalue (`KismetMathLibrary.Abs_Int` _returnvalue))))))
      (if (< (* _output_get _facedirection_y) 0.0)
        (set `self.CharacterState` "NewEnumerator2")
        (else
          (set `self.CharacterState` "NewEnumerator1")))
      (else
        (set `self.CharacterState` "NewEnumerator0")))
    (else
      (set `self.AttackInfoArray` _skillinfo_attackinfoarray)
      (set `self.AttackArrayIndex` 0)
      (`PaperZDAnimInstance.K2_PlayAnimationOverride` (`self.AnimBP`) _skillinfo_animseq "SkillSlot" 1.0 0.0))))

(fn `GetMoveRange`
  (returns (Min :type Integer) (Max :type Integer))
  (bind (_returnvalue_x _returnvalue_y) (`KismetMathLibrary.BreakVector` (`SceneComponent.K2_GetComponentLocation` (`self.CapsuleComponent`))))
  (return (`KismetMathLibrary.Max` (`KismetMathLibrary.FTrunc` (/ (- (`self.MinY`) _returnvalue_y) (`self.MoveStep`))) -6) (`KismetMathLibrary.Min` (`KismetMathLibrary.FTrunc` (/ (- (`self.MaxY`) _returnvalue_y) (`self.MoveStep`))) 6)))

(fn `Init`
  (params (InitInfo :type "/Game/Gameplay/Characters/S_CharacterInitInfo Structure"))
  (bind _sprite (`self.Sprite`))
  (set `self.GameDirector` InitInfo_GameDirector_19_190609674C39A232F4A4AA82F38E6D9F)
  (if InitInfo_IsLeft_6_CE0BA617491B17EE392198970854EB00
    (set `self.FaceDirection` (0.0 -1.0 0.0))
    (else
      (set `self.FaceDirection` (0.0 1.0 0.0))))
  (set `self.MinY` InitInfo_MinY_12_E6269C4D4BC4FD3022232EA61732776A)
  (set `self.MaxY` InitInfo_MaxY_13_1AB3482F4DDECCDFFD96D79A3A1B5AE3)
  (set `self.CharacterType` InitInfo_CharacterType_2_57C2CE154A6197D1504F04992F34CF1E)
  (bind _asabp_anim_bp (cast `/Game/Gameplay/Characters/ABP_AnimBP` (`PaperZDAnimationComponent.AnimInstance` (`self.AnimationComponent`))))
  (bind _output_get (set `self.AnimBP` _asabp_anim_bp))
  (`/Game/Gameplay/Characters/ABP_AnimBP.Init` _output_get self)
  (bind _output_get_2 (set `self.MaxHealth` 70.0))
  (set `self.CurrentHealth` _output_get_2)
  (bind _output_get_3 (set `self.MaxRenValue` 20.0))
  (set `self.CurrentRenValue` _output_get_3)
  (if (`|EnumEquality` (`self.CharacterType`) "NewEnumerator2")
    (`SceneComponent.K2_SetRelativeRotation` _sprite (struct :`Yaw` 180.0) false false)
    (`SceneComponent.SetRelativeScale3D` _sprite (0.85 0.85 0.85))
    (`SceneComponent.K2_SetRelativeLocation` _sprite (0.0 0.0 -45.0) false false)))

(fn `SaveAttackInfo`
  (bind _attackarrayindex (`self.AttackArrayIndex`))
  (set `self.AttackInfo` (`|GetArrayItem` (`self.AttackInfoArray`) _attackarrayindex))
  (set `self.AttackArrayIndex` (+ _attackarrayindex 1)))

(fn `SetRen`
  (params (DeltaRen :type "Float (double-precision)"))
  (returns (NewRen :type "Float (double-precision)"))
  (bind _output_get (set `self.CurrentRenValue` (`KismetMathLibrary.FClamp` (+ (`self.CurrentRenValue`) DeltaRen) 0.0 (`self.MaxRenValue`))))
  (return _output_get))

(fn `Stop`
  (params (Flag :type Boolean))
  (bind _returnvalue (`PaperZDAnimInstance.GetPlayer` (`PaperZDAnimationComponent.AnimInstance` (`self.AnimationComponent`))))
  (bind _output_get (set `self.HasStop` Flag))
  (if _output_get
    (`PaperZDAnimPlayer.PausePlayback` _returnvalue)
    (else
      (`PaperZDAnimPlayer.ResumePlayback` _returnvalue))))

(fn `StopMontage`
  (`PaperZDAnimInstance.StopAllAnimationOverrides` (`self.AnimBP`)))

(fn `UpdateMove`
  (params (DeltaTime :type "Float (double-precision)"))
  (`self.K2_SetActorLocation` (+ (`KismetMathLibrary.MakeVector` 0.0 (* DeltaTime (`self.MoveSpeed`))) (`self.K2_GetActorLocation`))))

(fn `UserConstructionScript`)