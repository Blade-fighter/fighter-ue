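; BP_CardInfo is a lookup for card data, serving each card's info, skill and UI by name.
; GetCardInfo searches the NameToCardInfo map and prints an error string when the name is missing.
; GetSkillInfo and GetCardUI build on it, with the skill picked from the card's SkillArray using the CharacterType value as the index.
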(fn `Get Skill Info`
  (params (SkillName :type String) (CharacterType :type "/Game/Gameplay/Characters/E_CharacterType Enum" :default "NewEnumerator0"))
  (returns (SkillInfo :type "/Game/Gameplay/Cards/Skills/S_SkillInfo Structure"))
  (return (`|GetArrayItem` (`.SkillArray_11_6D39554D49C506FB88659DA6E527B555` (break `/Game/Gameplay/Cards/S_CardInfo` (`self.GetCardInfo` SkillName))) (`KismetMathLibrary.Conv_ByteToInt` CharacterType))))

(fn `GetCardInfo`
  (params (CardName :type String))
  (returns (CardInfo :type "/Game/Gameplay/Cards/S_CardInfo Structure"))
  (bind (_value _returnvalue) (`BlueprintMapLibrary.Map_Find` (`self.NameToCardInfo`) CardName))
  (if _returnvalue
    (return _value)
    (else
      (`KismetSystemLibrary.PrintString` null "Fail To Get Exist CardInfo"))))

(fn `GetCardUI`
  (params (CardName :type String))
  (returns (CardUI :type "Texture2D Object Reference"))
  (bind (_cardinfo_name _cardinfo_cardui) (break `/Game/Gameplay/Cards/S_CardInfo` (`self.GetCardInfo` CardName)))
  (return _cardinfo_cardui))