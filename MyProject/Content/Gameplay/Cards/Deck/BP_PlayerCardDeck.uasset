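; BP_PlayerCardDeck is the player's card deck, linking card moves to the battle UI.
; It extends parent show functions so BattleWidget also shows cards moving from source to hand, by name, and from hand to discard, flagging whether the card was selected.
; Discarding requires both the parent check to pass and the card not to be the widget's locked index, so UI state gates deck logic.
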(fn `CanMoveHandToDiscard`
  (params (Index :type Integer))
  (returns (Result :type Boolean))
  (return (and (`parent.CanMoveHandToDiscard` Index) (!= (`/Game/Gameplay/UI/WB_BattleWidget.LockedIndex` (`self.BattleWidget`)) Index))))

(fn `MoveHandToDiscardShow`
  (params (Index :type Integer))
  (`parent.MoveHandToDiscardShow` Index)
  (`/Game/Gameplay/UI/WB_BattleWidget.MoveHandToDiscard` (`self.BattleWidget`) Index (== (`/Game/Gameplay/UI/WB_BattleWidget.SelectedIndex` (`self.BattleWidget`)) Index)))

(fn `MoveSourceToHandShow`
  (params (Index :type Integer))
  (`parent.MoveSourceToHandShow` Index)
  (`/Game/Gameplay/UI/WB_BattleWidget.MoveSourceToHand` (`self.BattleWidget`) Index (`|GetArrayItem` (`self.HandCards`) Index)))