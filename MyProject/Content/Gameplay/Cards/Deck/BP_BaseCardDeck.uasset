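; BP_BaseCardDeck is a base card deck that cycles cards between source, hand and discard piles.
; Init creates a capped set of hand slots, each paired with an empty flag.
; Empty slots draw from the top of the source pile, which refills from the shuffled discard pile when exhausted.
; Discarding frees slots, and empty Show functions act as hooks for presenting each move.
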(fn `CanMoveHandToDiscard`
  (params (Index :type Integer))
  (returns (Result :type Boolean))
  (return (not (`self.IsCardEmpty` Index))))

(fn `FilpCardEmpty`
  (params (Index :type Integer))
  (bind _handcardsempty (`self.HandCardsEmpty`))
  (`KismetArrayLibrary.Array_Set` _handcardsempty Index (not (`|GetArrayItem` _handcardsempty Index))))

(fn `Init`
  (params (SourceCards :type "Array of String"))
  (bind _output_get (set `self.SourceCards` SourceCards))
  (bind _output_get_2 (set `self.MaxHandCount` (`KismetMathLibrary.Min` (`KismetArrayLibrary.Array_Length` _output_get) 6)))
  (for _ (range _output_get_2)
    (`KismetArrayLibrary.Array_Add` (`self.HandCards`))
    (`KismetArrayLibrary.Array_Add` (`self.HandCardsEmpty`) true)))

(fn `IsCardEmpty`
  (params (Index :type Integer))
  (returns (IsEmpty :type Boolean))
  (return (`|GetArrayItem` (`self.HandCardsEmpty`) Index)))

(fn `MoveDiscardToSource`
  (bind _discardcards (`self.DiscardCards`))
  (`KismetArrayLibrary.Array_Shuffle` _discardcards)
  (set `self.SourceCards` _discardcards)
  (`KismetArrayLibrary.Array_Clear` (`self.DiscardCards`)))

(fn `MoveHandToDiscard`
  (for (_ _array_index) (`self.HandCards`)
    (`self.MoveHandToDiscardImpl` _array_index)))

(fn `MoveHandToDiscardImpl`
  (params (Index :type Integer) (ForceMove :type Boolean))
  (if (or (`self.CanMoveHandToDiscard` Index) ForceMove)
    (`self.FilpCardEmpty` Index)
    (`KismetArrayLibrary.Array_Add` (`self.DiscardCards`) (`|GetArrayItem` (`self.HandCards`) Index))
    (`self.MoveHandToDiscardShow` Index)))

(fn `MoveHandToDiscardShow`
  (params (Index :type Integer) (IsSelected :type Boolean)))

(fn `MoveSourceToHand`
  (bind _sourcecards (`self.SourceCards`))
  (for (_array_element _array_index) (`self.HandCardsEmpty`)
    (if _array_element
      (if (`KismetArrayLibrary.Array_IsEmpty` (`self.SourceCards`))
        (`self.MoveDiscardToSource`))
      (`KismetArrayLibrary.Array_Set` (`self.HandCards`) _array_index (`|GetArrayItem` _sourcecards))
      (`KismetArrayLibrary.Array_Remove` _sourcecards)
      (`self.FilpCardEmpty` _array_index)
      (`self.MoveSourceToHandShow` _array_index))))

(fn `MoveSourceToHandShow`
  (params (Index :type Integer)))