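; Animated battlefield background that scrolls trees, three M layers and sky at per-layer parallax speeds when UpdateMove runs.
; Tick uses random timers to launch pooled boats, clouds and birds along Y, marking idle ones by near-zero speed.
; Components passing the Y limit reset with random height and return to idle.
; BirdFly separately launches FlyingBird upward from a given Y with random drift until it clears a height limit.
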(event `self.ReceiveBeginPlay`
  (bind _movingboat (`self.MovingBoat`))
  (bind _movingcloud (`self.MovingCloud`))
  (bind _movingbird (`self.MovingBird`))
  (bind (_returnvalue_x _returnvalue_y _returnvalue_z) (`KismetMathLibrary.BreakVector` (`SceneComponent.K2_GetComponentLocation` (`self.FlyingBird`))))
  (`KismetArrayLibrary.Array_Add` _movingboat (`self.Boat1`))
  (`KismetArrayLibrary.Array_Add` _movingboat (`self.Boat2`))
  (`KismetArrayLibrary.Array_Add` _movingcloud (`self.cloud1`))
  (`KismetArrayLibrary.Array_Add` _movingcloud (`self.cloud2`))
  (set `self.BirdWorldZ` _returnvalue_z)
  (`KismetArrayLibrary.Array_Add` _movingbird (`self.bird1`))
  (`KismetArrayLibrary.Array_Add` _movingbird (`self.bird2`))
  (`KismetArrayLibrary.Array_Add` _movingbird (`self.bird3`)))

(event `self.ReceiveTick`
  (params (DeltaSeconds :type "Float (single-precision)"))
  (`self.Spawn Boat` DeltaSeconds)
  (`self.Spawn Cloud` DeltaSeconds)
  (`self.UpdateBoatAndCloud` DeltaSeconds)
  (`self.UpdateBird` DeltaSeconds)
  (`self.SpawnBird` DeltaSeconds)
  (`self.UpdateBirdMovingImpl` DeltaSeconds))

(fn `BirdFly`
  (params (WorldLocation :type "Vector Structure"))
  (bind _flyingbird (`self.FlyingBird`))
  (bind _returnvalue_x (`KismetMathLibrary.BreakVector` (`SceneComponent.K2_GetComponentLocation` _flyingbird)))
  (`parent.BirdFly` WorldLocation)
  (if (not (`self.bBirdFly`))
    (`SceneComponent.K2_SetWorldLocation` _flyingbird (`KismetMathLibrary.MakeVector` _returnvalue_x (.y WorldLocation) (`self.BirdWorldZ`)) false false)
    (set `self.BirdSpeed` (`KismetMathLibrary.MakeVector` 0.0 (`KismetMathLibrary.RandomFloatInRange` -200.0 200.0) 500.0))
    (set `self.bBirdFly` true)))

(fn `Spawn Boat`
  (params (DeltaTime :type "Float (double-precision)"))
  (if (<= (`self.BoatTime`) 0.001)
    (`self.SpawnMoving` true)
    (set `self.BoatTime` (`KismetMathLibrary.RandomFloatInRange` 3.0 6.0))
    (else
      (set `self.BoatTime` (- (`self.BoatTime`) DeltaTime)))))

(fn `Spawn Cloud`
  (params (DeltaTime :type "Float (double-precision)"))
  (if (<= (`self.CloudTime`) 0.001)
    (`self.SpawnMoving` false)
    (set `self.CloudTime` (`KismetMathLibrary.RandomFloatInRange` 1.0 3.0))
    (else
      (set `self.CloudTime` (- (`self.CloudTime`) DeltaTime)))))

(fn `SpawnBird`
  (params (DeltaTime :type "Float (double-precision)"))
  (bind _birdtime (`self.BirdTime`))
  (if (<= _birdtime 0.001)
    (`self.SpawnBirdImpl`)
    (set `self.BirdTime` (`KismetMathLibrary.RandomFloatInRange` 3.0 6.0))
    (else
      (set `self.BirdTime` (- _birdtime DeltaTime)))))

(fn `SpawnBirdImpl`
  (locals (Index :type Integer))
  (bind _index (`local.Index`))
  (for (_array_element _array_index) (`self.MovingBirdSpeed`)
    (if (< _array_element 0.1)
      (set `local.Index` _array_index)))
  (if (!= _index -1)
    (`KismetArrayLibrary.Array_Set` (`self.MovingBirdSpeed`) _index (`KismetMathLibrary.RandomFloatInRange` 40.0 80.0))))

(fn `SpawnMoving`
  (params (IsBoat :type Boolean))
  (locals (Index :type Integer :default -1))
  (bind _index (`local.Index`))
  (bind _index_2 (`local.Index`))
  (if IsBoat
    (for (_array_element _array_index) (`self.MovingBoatSpeed`)
      (if (< _array_element 0.1)
        (set `local.Index` _array_index)))
    (if (!= _index_2 -1)
      (`KismetArrayLibrary.Array_Set` (`self.MovingBoatSpeed`) _index_2 (`KismetMathLibrary.RandomFloatInRange` 35.0 45.0)))
    (else
      (for (_array_element_2 _array_index_2) (`self.MovingCloudSpeed`)
        (if (< _array_element_2 0.1)
          (set `local.Index` _array_index_2)))
      (if (!= _index -1)
        (`KismetArrayLibrary.Array_Set` (`self.MovingCloudSpeed`) _index (`KismetMathLibrary.RandomFloatInRange` 40.0 60.0))))))

(fn `UpdateBird`
  (params (DeltaTime :type "Float (double-precision)"))
  (bind _flyingbird (`self.FlyingBird`))
  (bind (_returnvalue_x _returnvalue_y _returnvalue_z) (`KismetMathLibrary.BreakVector` (`SceneComponent.K2_GetComponentLocation` _flyingbird)))
  (if (`self.bBirdFly`)
    (if (> _returnvalue_z 240.0)
      (set `self.bBirdFly` false)
      (else
        (`SceneComponent.K2_SetWorldLocation` _flyingbird (+ (* (`self.BirdSpeed`) DeltaTime) (`SceneComponent.K2_GetComponentLocation` _flyingbird)) false false)))))

(fn `UpdateBirdMoving`
  (params (DeltaTime :type "Float (double-precision)"))
  (returns (OutIndex :type "Array of Integer"))
  (locals (ResultIndex :type "Array of Integer"))
  (for (_array_element _array_index) (`self.MovingBirdSpeed`)
    (if (> _array_element 0.1)
      (bind _output (`|GetArrayItem` (`self.MovingBird`) _array_index))
      (bind (_returnvalue_x _returnvalue_y _returnvalue_z) (`KismetMathLibrary.BreakVector` (`SceneComponent.K2_GetComponentLocation` _output)))
      (`SceneComponent.K2_SetWorldLocation` _output (`KismetMathLibrary.MakeVector` _returnvalue_x (+ _returnvalue_y (* _array_element DeltaTime)) _returnvalue_z) false false)
      (bind (_returnvalue_x_2 _returnvalue_y_2) (`KismetMathLibrary.BreakVector` (`SceneComponent.K2_GetComponentLocation` _output)))
      (if (> _returnvalue_y_2 1000.0)
        (`KismetArrayLibrary.Array_Add` (`local.ResultIndex`) _array_index))))
  (return (`local.ResultIndex`)))

(fn `UpdateBirdMovingImpl`
  (params (DeltaTime :type "Float (double-precision)"))
  (bind _outindex (`self.UpdateBirdMoving` DeltaTime))
  (for _array_element _outindex
    (`SceneComponent.K2_SetRelativeLocation` (`|GetArrayItem` (`self.MovingBird`) _array_element) (`KismetMathLibrary.MakeVector` 0.0 0.0 (`KismetMathLibrary.RandomFloatInRange` -20.0 20.0)) false false)
    (`KismetArrayLibrary.Array_Set` (`self.MovingBirdSpeed`) _array_element)))

(fn `UpdateBoatAndCloud`
  (params (DeltaTime :type "Float (double-precision)"))
  (bind _outindex (`self.UpdateMoving` DeltaTime (`self.Cloud`) (`self.MovingCloudSpeed`) (`self.MovingCloud`)))
  (for _array_element _outindex
    (`SceneComponent.K2_SetRelativeLocation` (`|GetArrayItem` (`self.MovingCloud`) _array_element) (`KismetMathLibrary.MakeVector` 0.0 0.0 (`KismetMathLibrary.RandomFloatInRange` -20.0 20.0)) false false)
    (`KismetArrayLibrary.Array_Set` (`self.MovingCloudSpeed`) _array_element))
  (bind _outindex_2 (`self.UpdateMoving` DeltaTime (`self.Boat`) (`self.MovingBoatSpeed`) (`self.MovingBoat`)))
  (for _array_element_2 _outindex_2
    (`SceneComponent.K2_SetRelativeLocation` (`|GetArrayItem` (`self.MovingBoat`) _array_element_2) (`KismetMathLibrary.MakeVector` 0.0 0.0 (`KismetMathLibrary.RandomFloatInRange` -20.0 20.0)) false false)
    (`KismetArrayLibrary.Array_Set` (`self.MovingBoatSpeed`) _array_element_2)))

(fn `UpdateLayer`
  (params (SceneComp :type "SceneComponent Object Reference") (layer :type Integer) (Distance :type "Float (double-precision)"))
  (bind (_relativelocation_x _relativelocation_y _relativelocation_z) (`KismetMathLibrary.BreakVector` (`SceneComponent.RelativeLocation` SceneComp)))
  (`SceneComponent.K2_SetRelativeLocation` SceneComp (`KismetMathLibrary.MakeVector` _relativelocation_x (+ _relativelocation_y (* Distance (`|GetArrayItem` (`self.SpeedArray`) layer))) _relativelocation_z) false false))

(fn `UpdateMove`
  (params (DeltaTime :type "Float (double-precision)") (DeltaDistance :type "Float (double-precision)"))
  (bind _deltadistance (`local.DeltaDistance`))
  (`parent.UpdateMove` DeltaTime DeltaDistance)
  (`self.UpdateLayer` (`self.tree`) 0 DeltaDistance)
  (`self.UpdateLayer` (`self.m1`) 2 DeltaDistance)
  (`self.UpdateLayer` (`self.m2`) 3 _deltadistance)
  (`self.UpdateLayer` (`self.m3`) 5 _deltadistance)
  (`self.UpdateLayer` (`self.sky`) 7 _deltadistance))

(fn `UpdateMoving`
  (params (DeltaTime :type "Float (double-precision)") (SourceComponent :type "SceneComponent Object Reference") (SpeedArray :type "Array of Float (double-precision)") (CompArray :type "Array of PaperSpriteComponent Object Reference"))
  (returns (OutIndex :type "Array of Integer"))
  (locals (ResultIndex :type "Array of Integer"))
  (for (_array_element _array_index) SpeedArray
    (if (> _array_element 0.1)
      (bind _output (`|GetArrayItem` CompArray _array_index))
      (bind (_returnvalue_x _returnvalue_y _returnvalue_z) (`KismetMathLibrary.BreakVector` (`SceneComponent.K2_GetComponentLocation` _output)))
      (`SceneComponent.K2_SetWorldLocation` _output (`KismetMathLibrary.MakeVector` _returnvalue_x (+ _returnvalue_y (* _array_element DeltaTime)) _returnvalue_z) false false)
      (bind (_returnvalue_x_2 _returnvalue_y_2) (`KismetMathLibrary.BreakVector` (`SceneComponent.K2_GetComponentLocation` _output)))
      (if (> _returnvalue_y_2 1000.0)
        (`KismetArrayLibrary.Array_Add` (`local.ResultIndex`) _array_index))))
  (return (`local.ResultIndex`)))

(fn `UserConstructionScript`
  (`parent.UserConstructionScript`))