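; BP_PlayerMaster is the player-controlled battle master, extending a parent master with the player's card deck and battle UI hookup.
; Init builds a BP_PlayerCardDeck from the source cards, links it and itself to the battle widget, and enables start.
; NextKeImpl moves source cards to hand, and NextAction re-enables start when the parent returns false.
; ExecuteCommand sets a flag that makes MyUpdate skip its next parent update.
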(fn `ExecuteCommand`
  (params (Command :type String))
  (`parent.ExecuteCommand` Command)
  (set `self.IgnoreUpdate` true))

(fn `Init`
  (params (BaseCharacter :type "/Game/Gameplay/Characters/BP_BaseCharacter Object Reference") (SourceCards :type "Array of String (by ref)") (BattleWidget :type "/Game/Gameplay/UI/WB_BattleWidget Object Reference") (IsLeft :type Boolean) (BattleField :type "/Game/Gameplay/BattleFields/BattleField Object Reference"))
  (`parent.Init` BaseCharacter SourceCards BattleWidget IsLeft BattleField)
  (bind _returnvalue (`|GenericCreateObject` "/Game/Gameplay/Cards/Deck/BP_PlayerCardDeck.BP_PlayerCardDeck_C"))
  (bind _output_get (set `self.PlayerCardDeck` _returnvalue))
  (set `/Game/Gameplay/UI/WB_BattleWidget.PlayerCardDeck` _output_get BattleWidget)
  (set `/Game/Gameplay/UI/WB_BattleWidget.PlayerMaster` self BattleWidget)
  (`/Game/Gameplay/Cards/Deck/BP_BaseCardDeck.Init` _output_get SourceCards BattleWidget)
  (set `/Game/Gameplay/UI/WB_BattleWidget.CanStart` true (`self.Battle Widget`))
  (return))

(fn `MyUpdate`
  (params (DeltaTime :type "Float (double-precision)"))
  (if (`self.IgnoreUpdate`)
    (set `self.IgnoreUpdate` false)
    (else
      (`parent.MyUpdate` DeltaTime))))

(fn `NextAction`
  (bind _usecache (`parent.NextAction`))
  (if (not _usecache)
    (set `/Game/Gameplay/UI/WB_BattleWidget.CanStart` true (`self.Battle Widget`))))

(fn `NextKeImpl`
  (`parent.NextKeImpl`)
  (`/Game/Gameplay/Cards/Deck/BP_BaseCardDeck.MoveSourceToHand` (`self.PlayerCardDeck`)))

(fn `UserConstructionScript`
  (`parent.UserConstructionScript`))