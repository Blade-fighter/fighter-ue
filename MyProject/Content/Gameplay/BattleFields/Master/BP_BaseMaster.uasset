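; Base battle master that drives one side's character in a battlefield where actions are timed in Ke units.
; ExecuteCommand converts a command into a Ke cost and resumes the battlefield, while MyUpdate counts it down, restoring Ren each Ke.
; When time expires, NextAction stops the battlefield and resets character state.
; Attack and block reactions interrupt immediately, knockdown is cached until the next action, and NextKeImpl is an empty per-Ke hook.
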(fn `ClearState`
  (bind _basecharacter (`self.BaseCharacter`))
  (`/Game/Gameplay/Characters/BP_BaseCharacter.StopMontage` _basecharacter)
  (set `/Game/Gameplay/Characters/BP_BaseCharacter.MoveSpeed` 0.0 _basecharacter))

(fn `Equal`
  (params (A :type "Float (double-precision)") (B :type "Float (double-precision)"))
  (returns (Result :type Boolean))
  (return (< (`KismetMathLibrary.Abs` (- A B)) (`self.FloatError`))))

(fn `ExecuteCommand`
  (params (Command :type String))
  (bind _integer (`self.GetKe` Command))
  (`KismetArrayLibrary.Array_Add` (`self.Commands`) Command)
  (`/Game/Gameplay/UI/WB_BattleWidget.ChangeKe` (`self.Battle Widget`) _integer (`self.IsLeft`))
  (`self.SetKe` _integer)
  (`/Game/Gameplay/BattleFields/BattleField.Stop` (`self.BattleField`) false)
  (`/Game/Gameplay/Characters/BP_BaseCharacter.ExecuteCommand` (`self.BaseCharacter`) Command))

(fn `GetKe`
  (params (Name :type String))
  (returns (Integer :type Integer))
  (bind _returnvalue (`KismetMathLibrary.Abs_Int` (`KismetStringLibrary.Conv_StringToInt` Name)))
  (bind (_skillinfo_animseq _skillinfo_ke) (break `/Game/Gameplay/Cards/Skills/S_SkillInfo` (`/Game/Gameplay/Cards/BP_CardInfo.Get Skill Info` (`/Game/Gameplay/Director/GameDirector.TotalCardInfo` (`/Game/Gameplay/BattleFields/BattleField.GameDirector` (`self.BattleField`))) Name (`/Game/Gameplay/Characters/BP_BaseCharacter.CharacterType` (`self.BaseCharacter`)))))
  (if (`KismetStringLibrary.IsNumeric` Name)
    (if (== _returnvalue 0)
      (return 1)
      (else
        (return _returnvalue)))
    (else
      (return _skillinfo_ke))))

(fn `Init`
  (params (BaseCharacter :type "/Game/Gameplay/Characters/BP_BaseCharacter Object Reference") (SourceCards :type "Array of String") (BattleWidget :type "/Game/Gameplay/UI/WB_BattleWidget Object Reference") (IsLeft :type Boolean) (BattleField :type "/Game/Gameplay/BattleFields/BattleField Object Reference"))
  (set `self.BaseCharacter` BaseCharacter)
  (set `self.Battle Widget` BattleWidget)
  (set `self.IsLeft` IsLeft)
  (set `self.BattleField` BattleField))

(fn `InsertDown`
  (`self.ClearState`)
  (set `/Game/Gameplay/Characters/BP_BaseCharacter.CharacterState` "NewEnumerator7" (`self.BaseCharacter`))
  (`/Game/Gameplay/UI/WB_BattleWidget.ChangeKe` (`self.Battle Widget`) 3 (`self.IsLeft`))
  (`self.SetKe` 3)
  (`/Game/Gameplay/BattleFields/BattleField.Stop` (`self.BattleField`) false))

(fn `InsertState`
  (params (State :type "/Game/Gameplay/BattleFields/Master/E_InsertState Enum" :default "NewEnumerator0"))
  (switch `/Game/Gameplay/BattleFields/Master/E_InsertState` State
    (:`NewEnumerator1`
      (`self.InsertTempState` "NewEnumerator4")
      (`/Game/Gameplay/Characters/ABP_AnimBP.RandomAttackedIndex` (`/Game/Gameplay/Characters/BP_BaseCharacter.AnimBP` (`self.BaseCharacter`))))
    (:`NewEnumerator2`
      (set `self.CacheInsertState` "NewEnumerator2"))
    (:`NewEnumerator3`
      (`self.InsertTempState` "NewEnumerator3"))))

(fn `InsertTempState`
  (params (State :type "/Game/Gameplay/Characters/E_CharacterState Enum" :default "NewEnumerator0"))
  (bind _basecharacter (`self.BaseCharacter`))
  (`self.ClearState`)
  (`/Game/Gameplay/Characters/BP_BaseCharacter.ChangeFaceDirection` _basecharacter)
  (set `/Game/Gameplay/Characters/BP_BaseCharacter.CharacterState` State _basecharacter)
  (`self.SetKe` 1)
  (`/Game/Gameplay/UI/WB_BattleWidget.ChangeKe` (`self.Battle Widget`) 1 (`self.IsLeft`)))

(fn `MyUpdate`
  (params (DeltaTime :type "Float (double-precision)"))
  (locals (LastKe :type Integer))
  (bind _keinterval (`self.KeInterval`))
  (if (not (`self.HasEnd`))
    (`/Game/Gameplay/Characters/BP_BaseCharacter.MyUpdate` (`self.BaseCharacter`) DeltaTime)
    (if (`self.DelayAction`)
      (`self.NextAction`)
      (set `self.DelayAction` false)
      (else
        (bind _output_get (set `self.LeftTime` (- (`self.LeftTime`) DeltaTime)))
        (if (`self.Equal` (mod _output_get _keinterval) (`local.DeltaTime`))
          (`self.NextKe` (`KismetMathLibrary.FTrunc` (/ _output_get _keinterval))))
        (if (`self.Equal` (`self.LeftTime`) (`local.DeltaTime`))
          (set `self.DelayAction` true))))))

(fn `NextAction`
  (returns (UseCache :type Boolean))
  (if (not (`self.HasEnd`))
    (`/Game/Gameplay/Characters/BP_BaseCharacter.ChangeFaceDirection` (`self.BaseCharacter`))
    (`/Game/Gameplay/BattleFields/BattleField.Stop` (`self.BattleField`) true)
    (`self.ResetCharacterState`)
    (if (`|EnumInequality` (`self.CacheInsertState`) "NewEnumerator0")
      (switch `/Game/Gameplay/BattleFields/Master/E_InsertState` (`self.CacheInsertState`)
        (:`NewEnumerator2`
          (`self.InsertDown`)
          (set `self.CacheInsertState` "NewEnumerator0")
          (return true)))
      (else
        (return false)))))

(fn `NextKe`
  (params (NewKe :type Integer))
  (`/Game/Gameplay/UI/WB_BattleWidget.ChangeKe` (`self.Battle Widget`) NewKe (`self.IsLeft`))
  (`/Game/Gameplay/Characters/BP_BaseCharacter.SetRen` (`self.BaseCharacter`) (`self.RenUpValue`))
  (`self.NextKeImpl`))

(fn `NextKeImpl`)

(fn `ResetCharacterState`
  (bind _basecharacter (`self.BaseCharacter`))
  (if (`|EnumEquality` (`/Game/Gameplay/Characters/BP_BaseCharacter.CharacterState` _basecharacter) "NewEnumerator7")
    (`/Game/Gameplay/Characters/BP_BaseCharacter.SetRen` _basecharacter (`/Game/Gameplay/Characters/BP_BaseCharacter.MaxRenValue` _basecharacter)))
  (set `/Game/Gameplay/Characters/BP_BaseCharacter.CharacterState` "NewEnumerator0" _basecharacter)
  (set `/Game/Gameplay/Characters/BP_BaseCharacter.MoveSpeed` 0.0 (`self.BaseCharacter`)))

(fn `SetKe`
  (params (Ke :type Integer))
  (set `self.LeftTime` (* Ke (`self.KeInterval`))))

(fn `UserConstructionScript`)