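; BP_AIMaster is the AI-controlled battlefield master, extending its parent's turn flow with automatic command choice.
; Init creates its own card deck from the source cards, and NextKeImpl moves cards from source to hand.
; When the parent's NextAction returns false, it executes an AI command, then discards the hand.
; The command is usually the first hand card, with about a 20% chance of a random value within the character's move range.
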(event `self.ReceiveTick`
  (params (DeltaSeconds :type "Float (single-precision)")))

(fn `EnemyAI`
  (returns (Result :type String))
  (bind (_min _max) (`/Game/Gameplay/Characters/BP_BaseCharacter.GetMoveRange` (`self.BaseCharacter`)))
  (if (> (`KismetMathLibrary.RandomFloat`) 0.8)
    (return (`KismetStringLibrary.Conv_IntToString` (`KismetMathLibrary.RandomIntegerInRange` _min _max)))
    (else
      (return (`|GetArrayItem` (`/Game/Gameplay/Cards/Deck/BP_BaseCardDeck.HandCards` (`self.BaseCardDeck`)))))))

(fn `Init`
  (params (BaseCharacter :type "/Game/Gameplay/Characters/BP_BaseCharacter Object Reference") (SourceCards :type "Array of String (by ref)") (BattleWidget :type "/Game/Gameplay/UI/WB_BattleWidget Object Reference") (IsLeft :type Boolean) (BattleField :type "/Game/Gameplay/BattleFields/BattleField Object Reference"))
  (`parent.Init` BaseCharacter SourceCards BattleWidget IsLeft BattleField)
  (bind _returnvalue (`|GenericCreateObject` "/Game/Gameplay/Cards/Deck/BP_BaseCardDeck.BP_BaseCardDeck_C"))
  (bind _output_get (set `self.BaseCardDeck` _returnvalue))
  (`/Game/Gameplay/Cards/Deck/BP_BaseCardDeck.Init` _output_get SourceCards BattleWidget)
  (`/Game/Gameplay/UI/WB_BattleWidget.PlayNormalHead` BattleWidget)
  (return))

(fn `NextAction`
  (bind _usecache (`parent.NextAction`))
  (if (not _usecache)
    (bind _result (`self.EnemyAI`))
    (`self.ExecuteCommand` _result)
    (`/Game/Gameplay/Cards/Deck/BP_BaseCardDeck.MoveHandToDiscard` (`self.BaseCardDeck`))))

(fn `NextKeImpl`
  (`parent.NextKeImpl`)
  (`/Game/Gameplay/Cards/Deck/BP_BaseCardDeck.MoveSourceToHand` (`self.BaseCardDeck`)))

(fn `UserConstructionScript`
  (`parent.UserConstructionScript`))